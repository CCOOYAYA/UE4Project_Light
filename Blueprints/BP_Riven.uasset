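; BP_Riven is a pickup that rolls random Riven stat modifiers across Health, AttackPower, CriticalHit and EfficiencyofLP.
; BeginPlay picks a positive/negative pattern through cascaded random rolls, with one to three affected stats.
; SetRivenData stores the values and counts signs.
; After a one-second collision delay, ThirdPersonCharacter overlap fills a W_Riven widget, adds it to the player's RivenWrapBox with the data, plays a sound and destroys the actor.
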(event OnComponentBeginOverlap(Box)
  (params (OverlappedComponent :type Primitive%20Component%20Object%20Reference) (OtherActor :type Actor%20Object%20Reference) (OtherComp :type Primitive%20Component%20Object%20Reference) (OtherBodyIndex :type Integer) (bFromSweep :type Boolean) (SweepResult :type Hit%20Result%20Structure%20%28by%20ref%29))
  (Utilities|Casting|CastToThirdPersonCharacter OtherActor)
  (Utilities|FlowControl|DoOnce false
    (:Completed
      (bind _returnvalue (UserInterface|CreateWidget "/Game/ThirdPersonBP/Blueprints/W_Riven.W_Riven_C"))
      (Variables|Default|SetWRiven _returnvalue)
      (if (== (Variables|Default|GetPositive) 0)
        (Default|SetRivenText (Variables|Default|GetWRiven) (Utilities|Text|ToText(String) (Utilities|String|Append "-" (Utilities|String|ToString(Integer) (Variables|Default|GetNegative)))))
        (elif (== (Variables|Default|GetNegative) 0)
          (Default|SetRivenText (Variables|Default|GetWRiven) (Utilities|Text|ToText(String) (Utilities|String|Append "+" (Utilities|String|ToString(Integer) (Variables|Default|GetPositive)))))
          (else
            (Default|SetRivenText (Variables|Default|GetWRiven) (Utilities|Text|ToText(String) (Utilities|String|Append "+" (Utilities|String|ToString(Integer) (Variables|Default|GetPositive)) "-" (Utilities|String|ToString(Integer) (Variables|Default|GetNegative))))))))
      (for (_array_element _array_index) (Variables|Default|GetRivenDataArray)
        (if (not (== _array_element 0.0))
          (bind _output_get (Variables|Default|SetTempValue (Math|Float|Round _array_element)))
          (Development|PrintString (Utilities|String|ToString(Integer) _output_get) false true "(R=0.000000,G=0.660000,B=1.000000,A=1.000000)" 2e+01)
          (switch int _array_index
            (:0
              (Default|SetRivenHealthText (Variables|Default|GetWRiven) (Utilities|Text|ToText(String) (Utilities|String|Append "Health : " (Utilities|String|ToString(Integer) (Variables|Default|GetTempValue))))))
            (:1
              (Default|SetRivenAttackPowerText (Variables|Default|GetWRiven) (Utilities|Text|ToText(String) (Utilities|String|Append "AttackPower : " (Utilities|String|ToString(Integer) (Variables|Default|GetTempValue))))))
            (:2
              (Default|SetRivenCriticalHitText (Variables|Default|GetWRiven) (Utilities|Text|ToText(String) (Utilities|String|Append "CriticalHit : " (Utilities|String|ToString(Integer) (Variables|Default|GetTempValue))))))
            (:3
              (Default|SetRivenEfficiencyofLPText (Variables|Default|GetWRiven) (Utilities|Text|ToText(String) (Utilities|String|Append "EofLP : " (Utilities|String|ToString(Integer) (Variables|Default|GetTempValue)))))))))
      (Widget|Panel|AddChild (Variables|/Game/ThirdPersonBP/Blueprints/W_IngameUI.W_IngameUI_C|GetRivenWrapBox (Variables|/Game/ThirdPersonBP/Blueprints/ThirdPersonCharacter.ThirdPersonCharacter_C|GetIngameUI (.AsThird%20Person%20Character (Utilities|Casting|CastToThirdPersonCharacter (Game|GetPlayerCharacter 0))))) (Variables|Default|GetWRiven))
      (Variables|/Game/ThirdPersonBP/Blueprints/W_Riven.W_Riven_C|SetisRiven (Variables|Default|GetWRiven) true)
      (Variables|/Game/ThirdPersonBP/Blueprints/W_Riven.W_Riven_C|SetCurrentRivenDS (Variables|Default|GetWRiven) (Variables|Default|GetRivenData))
      (Audio|PlaySound2D "/Game/Assets/Sounds/Character/A_Character_Heal01_Mana.A_Character_Heal01_Mana" 1.0 1.0 0.0 0 0)
      (Actor|DestroyActor))))

(event Custom|SetRivenData
  (params (Health :type Float%20%28single-precision%29) (AttackPower :type Float%20%28single-precision%29) (CriticalHit :type Float%20%28single-precision%29) (EfficiencyofLP :type Float%20%28single-precision%29))
  (bind _output_get (Variables|Default|SetHealth Health))
  (Utilities|Array|SetArrayElem (Variables|Default|GetRivenDataArray) 0 _output_get)
  (bind _output_get_2 (Variables|Default|SetAttackPower AttackPower))
  (Utilities|Array|SetArrayElem (Variables|Default|GetRivenDataArray) 1 _output_get_2)
  (bind _output_get_3 (Variables|Default|SetCriticalHit CriticalHit))
  (Utilities|Array|SetArrayElem (Variables|Default|GetRivenDataArray) 2 _output_get_3)
  (bind _output_get_4 (Variables|Default|SetEfficiencyofLP EfficiencyofLP))
  (Utilities|Array|SetArrayElem (Variables|Default|GetRivenDataArray) 3 _output_get_4)
  (Variables|Default|SetRivenData (Utilities|Struct|MakeRivenDataStruct (Variables|Default|GetHealth) (Variables|Default|GetAttackPower) (Variables|Default|GetCriticalHit) (Variables|Default|GetEfficiencyofLP)))
  (for _array_element (Variables|Default|GetRivenDataArray)
    (Development|PrintString (Utilities|String|ToString(Float) _array_element) false true "(R=0.000000,G=0.660000,B=1.000000,A=1.000000)" 2e+01)
    (Math|Float|CompareFloat _array_element 0.0
      (:>
        (Math|Integer|IncrementInt (Variables|Default|GetPositive)))
      (:<
        (Math|Integer|IncrementInt (Variables|Default|GetNegative)))))
  (Development|PrintString (Utilities|String|Append "P:" (Utilities|String|ToString(Integer) (Variables|Default|GetPositive)) "N:" (Utilities|String|ToString(Integer) (Variables|Default|GetNegative))) false true "(R=0.000000,G=0.660000,B=1.000000,A=1.000000)" 2e+01))

(event EventBeginPlay
  (bind _returnvalue (Math|Random|RandomFloatinRange 0.0 1e+01))
  (bind _returnvalue_2 (Math|Random|RandomIntegerinRange 0 2))
  (bind _returnvalue_3 (Math|Random|RandomIntegerinRange 0 2))
  (bind _returnvalue_4 (Math|Random|RandomIntegerinRange 0 2))
  (bind _returnvalue_5 (Math|Random|RandomIntegerinRange 0 5))
  (bind _returnvalue_6 (Math|Random|RandomIntegerinRange 0 5))
  (bind _returnvalue_7 (Math|Random|RandomIntegerinRange 0 1))
  (bind _returnvalue_8 (Math|Random|RandomIntegerinRange 0 1))
  (bind _returnvalue_9 (Math|Random|RandomIntegerinRange 0 1))
  (bind _returnvalue_10 (Math|Random|RandomIntegerinRange 0 1))
  (bind _returnvalue_11 (Math|Random|RandomIntegerinRange 0 1))
  (bind _returnvalue_12 (Math|Random|RandomIntegerinRange 0 1))
  (bind _returnvalue_13 (Math|Random|RandomIntegerinRange 0 3))
  (bind _returnvalue_14 (Math|Random|RandomIntegerinRange 0 2))
  (bind _box (Variables|Default|GetBox))
  (Utilities|FlowControl|Sequence
    (:then_0
      (Collision|SetCollisionEnabled _box "NoCollision")
      (Utilities|FlowControl|Delay 1.0)
      (Collision|SetCollisionEnabled _box "QueryAndPhysics"))
    (:then_1
      (Development|PrintString (Utilities|String|Append "first:" (Utilities|String|ToString(Float) _returnvalue)) false true "(R=0.000000,G=0.660000,B=1.000000,A=1.000000)" 2e+01)
      (if (< _returnvalue 2.0)
        ;[1 1 1] -1
        (switch int (Math|Random|RandomIntegerinRange 0 3)
          (:0
            (CallFunction|SetRivenData (Math|Random|RandomFloatinRange -2e+02 -1.0) 0.0 0.0 0.0))
          (:1
            (CallFunction|SetRivenData 0.0 (Math|Random|RandomFloatinRange -2e+01 -1.0) 0.0 0.0))
          (:2
            (CallFunction|SetRivenData 0.0 0.0 (Math|Random|RandomFloatinRange -1e+01 -1.0) 0.0))
          (:3
            (CallFunction|SetRivenData 0.0 0.0 0.0 (Math|Random|RandomFloatinRange -5e+01 -1.0))))
        (elif (< _returnvalue 5.0)
          ;[1 1 1] +1
          (switch int (Math|Random|RandomIntegerinRange 0 3)
            (:0
              (CallFunction|SetRivenData (Math|Random|RandomFloatinRange 1.0 2e+02) 0.0 0.0 0.0))
            (:1
              (CallFunction|SetRivenData 0.0 (Math|Random|RandomFloatinRange 1.0 2e+01) 0.0 0.0))
            (:2
              (CallFunction|SetRivenData 0.0 0.0 (Math|Random|RandomFloatinRange 1.0 1e+01) 0.0))
            (:3
              (CallFunction|SetRivenData 0.0 0.0 0.0 (Math|Random|RandomFloatinRange 1.0 5e+01))))
          (elif (< _returnvalue 8.0)
            (Development|PrintString (Utilities|String|ToString(Integer) _returnvalue_13) false true "(R=0.000000,G=0.660000,B=1.000000,A=1.000000)" 2e+01)
            ;[1 1 1] +1-1
            (switch int _returnvalue_13
              (:0
                (Development|PrintString (Utilities|String|ToString(Integer) _returnvalue_14) false true "(R=0.000000,G=0.660000,B=1.000000,A=1.000000)" 2e+01)
                (switch int _returnvalue_14
                  (:0
                    (CallFunction|SetRivenData (Math|Random|RandomFloatinRange 1.0 2e+02) (Math|Random|RandomFloatinRange -2e+01 -1.0) 0.0 0.0))
                  (:1
                    (CallFunction|SetRivenData (Math|Random|RandomFloatinRange 1.0 2e+02) 0.0 (Math|Random|RandomFloatinRange -1e+01 -1.0) 0.0))
                  (:2
                    (CallFunction|SetRivenData (Math|Random|RandomFloatinRange 1.0 2e+02) 0.0 0.0 (Math|Random|RandomFloatinRange -5e+01 -1.0)))))
              (:1
                (Development|PrintString (Utilities|String|ToString(Integer) _returnvalue_2) false true "(R=0.000000,G=0.660000,B=1.000000,A=1.000000)" 2e+01)
                (switch int _returnvalue_2
                  (:0
                    (CallFunction|SetRivenData (Math|Random|RandomFloatinRange -2e+02 -1.0) (Math|Random|RandomFloatinRange 1.0 2e+01) 0.0 0.0))
                  (:1
                    (CallFunction|SetRivenData 0.0 (Math|Random|RandomFloatinRange 1.0 2e+01) (Math|Random|RandomFloatinRange -1e+01 -1.0) 0.0))
                  (:2
                    (CallFunction|SetRivenData 0.0 (Math|Random|RandomFloatinRange 1.0 2e+01) 0.0 (Math|Random|RandomFloatinRange -5e+01 -1.0)))))
              (:2
                (Development|PrintString (Utilities|String|ToString(Integer) _returnvalue_3) true true "(R=0.000000,G=0.660000,B=1.000000,A=1.000000)" 2e+01)
                (switch int _returnvalue_3
                  (:0
                    (CallFunction|SetRivenData (Math|Random|RandomFloatinRange -2e+02 -1.0) 0.0 (Math|Random|RandomFloatinRange 1.0 1e+01) 0.0))
                  (:1
                    (CallFunction|SetRivenData 0.0 (Math|Random|RandomFloatinRange -2e+01 -1.0) (Math|Random|RandomFloatinRange 1.0 1e+01) 0.0))
                  (:2
                    (CallFunction|SetRivenData 0.0 0.0 (Math|Random|RandomFloatinRange 1.0 1e+01) (Math|Random|RandomFloatinRange -5e+01 -1.0)))))
              (:3
                (Development|PrintString (Utilities|String|ToString(Integer) _returnvalue_4) false true "(R=0.000000,G=0.660000,B=1.000000,A=1.000000)" 2e+01)
                (switch int _returnvalue_4
                  (:0
                    (CallFunction|SetRivenData (Math|Random|RandomFloatinRange -2e+02 -1.0) 0.0 0.0 (Math|Random|RandomFloatinRange 1.0 5e+01)))
                  (:1
                    (CallFunction|SetRivenData 0.0 (Math|Random|RandomFloatinRange -2e+01 -1.0) 0.0 (Math|Random|RandomFloatinRange 1.0 5e+01)))
                  (:2
                    (CallFunction|SetRivenData 0.0 0.0 (Math|Random|RandomFloatinRange -1e+01 -1.0) (Math|Random|RandomFloatinRange 1.0 5e+01))))))
            (elif (< _returnvalue 9.0)
              ;[1 1 1] +2
              (Development|PrintString (Utilities|String|ToString(Integer) _returnvalue_5) false true "(R=0.000000,G=0.660000,B=1.000000,A=1.000000)" 2e+01)
              (switch int _returnvalue_5
                (:0
                  (CallFunction|SetRivenData (Math|Random|RandomFloatinRange 1.0 2e+02) (Math|Random|RandomFloatinRange 1.0 2e+01) 0.0 0.0))
                (:1
                  (CallFunction|SetRivenData (Math|Random|RandomFloatinRange 1.0 2e+02) 0.0 (Math|Random|RandomFloatinRange 1.0 1e+01) 0.0))
                (:2
                  (CallFunction|SetRivenData (Math|Random|RandomFloatinRange 1.0 2e+02) 0.0 0.0 (Math|Random|RandomFloatinRange 1.0 5e+01)))
                (:3
                  (CallFunction|SetRivenData 0.0 (Math|Random|RandomFloatinRange 1.0 2e+01) (Math|Random|RandomFloatinRange 1.0 1e+01) 0.0))
                (:4
                  (CallFunction|SetRivenData 0.0 (Math|Random|RandomFloatinRange 1.0 2e+01) 0.0 (Math|Random|RandomFloatinRange 1.0 5e+01)))
                (:5
                  (CallFunction|SetRivenData 0.0 0.0 (Math|Random|RandomFloatinRange 1.0 1e+01) (Math|Random|RandomFloatinRange 1.0 5e+01))))
              (else
                ;[1 1 1] +2-1
                (Development|PrintString (Utilities|String|ToString(Integer) _returnvalue_6) true true "(R=0.000000,G=0.660000,B=1.000000,A=1.000000)" 2e+01)
                (switch int _returnvalue_6
                  (:0
                    (Development|PrintString (Utilities|String|ToString(Integer) _returnvalue_7) false true "(R=0.000000,G=0.660000,B=1.000000,A=1.000000)" 2e+01)
                    (switch int _returnvalue_7
                      (:0
                        (CallFunction|SetRivenData (Math|Random|RandomFloatinRange 1.0 2e+02) (Math|Random|RandomFloatinRange 1.0 2e+01) (Math|Random|RandomFloatinRange -1e+01 -1.0) 0.0))
                      (:1
                        (CallFunction|SetRivenData (Math|Random|RandomFloatinRange 1.0 2e+02) (Math|Random|RandomFloatinRange 1.0 2e+01) 0.0 (Math|Random|RandomFloatinRange -5e+01 -1.0)))))
                  (:1
                    (Development|PrintString (Utilities|String|ToString(Integer) _returnvalue_8) false true "(R=0.000000,G=0.660000,B=1.000000,A=1.000000)" 2e+01)
                    (switch int _returnvalue_8
                      (:0
                        (CallFunction|SetRivenData (Math|Random|RandomFloatinRange 1.0 2e+02) (Math|Random|RandomFloatinRange -2e+01 -1.0) (Math|Random|RandomFloatinRange 1.0 1e+01) 0.0))
                      (:1
                        (CallFunction|SetRivenData (Math|Random|RandomFloatinRange 1.0 2e+02) 0.0 (Math|Random|RandomFloatinRange 1.0 1e+01) (Math|Random|RandomFloatinRange -5e+01 -1.0)))))
                  (:2
                    (Development|PrintString (Utilities|String|ToString(Integer) _returnvalue_9) false true "(R=0.000000,G=0.660000,B=1.000000,A=1.000000)" 2e+01)
                    (switch int _returnvalue_9
                      (:0
                        (CallFunction|SetRivenData (Math|Random|RandomFloatinRange 1.0 2e+02) (Math|Random|RandomFloatinRange -2e+01 -1.0) 0.0 (Math|Random|RandomFloatinRange 1.0 5e+01)))
                      (:1
                        (CallFunction|SetRivenData (Math|Random|RandomFloatinRange 1.0 2e+02) 0.0 (Math|Random|RandomFloatinRange -1e+01 -1.0) (Math|Random|RandomFloatinRange 1.0 5e+01)))))
                  (:3
                    (Development|PrintString (Utilities|String|ToString(Integer) _returnvalue_10) false true "(R=0.000000,G=0.660000,B=1.000000,A=1.000000)" 2e+01)
                    (switch int _returnvalue_10
                      (:0
                        (CallFunction|SetRivenData (Math|Random|RandomFloatinRange -2e+02 -1.0) (Math|Random|RandomFloatinRange 1.0 2e+01) (Math|Random|RandomFloatinRange 1.0 1e+01) 0.0))
                      (:1
                        (CallFunction|SetRivenData 0.0 (Math|Random|RandomFloatinRange 1.0 2e+01) (Math|Random|RandomFloatinRange 1.0 1e+01) (Math|Random|RandomFloatinRange -5e+01 -1.0)))))
                  (:4
                    (Development|PrintString (Utilities|String|ToString(Integer) _returnvalue_11) false true "(R=0.000000,G=0.660000,B=1.000000,A=1.000000)" 2e+01)
                    (switch int _returnvalue_11
                      (:0
                        (CallFunction|SetRivenData (Math|Random|RandomFloatinRange -2e+02 -1.0) (Math|Random|RandomFloatinRange 1.0 2e+01) 0.0 (Math|Random|RandomFloatinRange 1.0 5e+01)))
                      (:1
                        (CallFunction|SetRivenData 0.0 (Math|Random|RandomFloatinRange 1.0 2e+01) (Math|Random|RandomFloatinRange -1e+01 -1.0) (Math|Random|RandomFloatinRange 1.0 5e+01)))))
                  (:5
                    (Development|PrintString (Utilities|String|ToString(Integer) _returnvalue_12) false true "(R=0.000000,G=0.660000,B=1.000000,A=1.000000)" 2e+01)
                    (switch int _returnvalue_12
                      (:0
                        (CallFunction|SetRivenData (Math|Random|RandomFloatinRange -2e+02 -1.0) 0.0 (Math|Random|RandomFloatinRange 1.0 1e+01) (Math|Random|RandomFloatinRange 1.0 5e+01)))
                      (:1
                        (CallFunction|SetRivenData 0.0 (Math|Random|RandomFloatinRange -2e+01 -1.0) (Math|Random|RandomFloatinRange 1.0 1e+01) (Math|Random|RandomFloatinRange 1.0 5e+01))))))))))))))

(event Collision|EventActorBeginOverlap
  (params (OtherActor :type Actor%20Object%20Reference)))

(event EventTick
  (params (DeltaSeconds :type Float%20%28single-precision%29)))

(fn ConstructionScript)