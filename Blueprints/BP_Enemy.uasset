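; Enemy AI character that patrols random navmesh points, chases the player on sight and drops pickups or actors on death.
; PawnSensing drives the chase, while Tick opens a timed AttackCapsule collision window when the player is near, after a random delay.
; Capsule overlaps damage ThirdPersonCharacter.
; AnyDamage updates HP text; death disables attacks, spawns BP_lightball plus random extra BP_lightball or BP_Riven, then destroys the actor after a delay.
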(event OnSeePawn(PawnSensing)
  (params (Pawn :type Pawn%20Object%20Reference))
  ;[1 1 1] 感知事件（基于PawnSensing组件），感知范围内的玩家，并向玩家靠近
  (if (Variables|Default|GetIsDead)
    ;;[1 1 1] 死亡后立即停止移动
    (Components|Movement|StopMovementImmediately (Variables|Character|GetCharacterMovement))
    (else
      (bind _asthird_person_character (Utilities|Casting|CastToThirdPersonCharacter Pawn)
        (:then
          (Variables|Default|SetChasing true)
          (if (not (Variables|Default|GetisAttacking))
            (AI|AIMoveTo (Class|PawnMovementComponent|GetPawnOwner (Variables|Character|GetCharacterMovement)) "0, 0, 0" _asthird_person_character 1.5e+02 false)))
        (:CastFailed
          (Variables|Default|SetChasing false)
          (CallFunction|Patrol))))))

(event OnComponentBeginOverlap(AttackCapsule)
  (params (OverlappedComponent :type Primitive%20Component%20Object%20Reference) (OtherActor :type Actor%20Object%20Reference) (OtherComp :type Primitive%20Component%20Object%20Reference) (OtherBodyIndex :type Integer) (bFromSweep :type Boolean) (SweepResult :type Hit%20Result%20Structure%20%28by%20ref%29))
  (bind _asthird_person_character (Utilities|Casting|CastToThirdPersonCharacter OtherActor))
  (Utilities|FlowControl|DoOnce false :!label _label
    (:Completed
      (Default|CountHealth _asthird_person_character (Variables|Default|GetEnemyDamage))
      (Utilities|FlowControl|Delay 0.5)
      (goto _label Reset))))

(event Custom|Patrol
  (if (not (Variables|Default|GetChasing)) :!label _label
    (Utilities|FlowControl|Delay 2.0)
    (bind _outactors (Actor|GetAllActorsOfClass "/Script/NavigationSystem.RecastNavMesh"))
    (AI|AIMoveTo self (.RandomLocation (Class|NavigationSystemV1|GetRandomPointinNavigableRadius (Transformation|GetActorLocation) 1e+03 (Utilities|Array|Get(acopy) _outactors) 0)) 0 1e+01 true
      (:OnSuccess
        (goto _label))
      (:OnFail
        (goto _label)))))

(event EventBeginPlay
  ;[1 1 1] 初始化敌人生命值，给AI角色一个控制器
  (Variables|Default|SetEnemyHP 4.5e+02)
  (Pawn|SpawnDefaultController)
  (CallFunction|Patrol)
  (Collision|SetCollisionEnabled (Variables|Default|GetAttackCapsule) "NoCollision"))

(event Game|Damage|EventAnyDamage
  (params (Damage :type Float%20%28single-precision%29) (DamageType :type Damage%20Type%20Object%20Reference) (InstigatedBy :type Controller%20Object%20Reference) (DamageCauser :type Actor%20Object%20Reference))
  (bind _returnvalue (Transformation|GetActorLocation))
  (bind _returnvalue_2 (Math|Random|RandomFloatinRange -1e+02 1e+02))
  (bind _returnvalue_3 (Transformation|GetActorLocation))
  (bind _returnvalue_4 (Math|Random|RandomFloatinRange -1e+02 1e+02))
  (bind _returnvalue_5 (Transformation|GetActorLocation))
  (bind _returnvalue_6 (Math|Random|RandomFloatinRange -1e+02 1e+02))
  (bind _returnvalue_7 (Transformation|GetActorLocation))
  (bind _returnvalue_8 (Math|Random|RandomFloatinRange -1e+02 1e+02))
  (bind _textrender (Variables|Default|GetTextRender))
  (bind (_x _y _z) (Math|Vector|BreakVector _returnvalue))
  (bind (_x_2 _y_2 _z_2) (Math|Vector|BreakVector _returnvalue_3))
  (bind (_x_3 _y_3 _z_3) (Math|Vector|BreakVector _returnvalue_5))
  (bind (_x_4 _y_4 _z_4) (Math|Vector|BreakVector _returnvalue_7))
  (if (not (Variables|Default|GetIsDead))
    (bind _output_get (Variables|Default|SetEnemyHP (- (Variables|Default|GetEnemyHP) Damage)))
    (Rendering|Components|TextRender|SetText _textrender (Utilities|Text|ToText(String) (Class|KismetMathLibrary|FTrunc64 _output_get)))
    (if (<= _output_get 0.0)
      (Rendering|SetVisibility _textrender false false)
      (Utilities|FlowControl|DoOnce false
        (:Completed
          (Collision|SetCollisionEnabled (Variables|Default|GetAttackCapsule) "NoCollision")
          (Variables|Default|SetIsDead (<= _output_get 0.0))
          (Game|SpawnActorfromClass "/Game/ThirdPersonBP/Blueprints/BP_lightball.BP_lightball_C" (Math|Transform|MakeTransform (Math|Vector|MakeVector (+ _x_3 _returnvalue_6) (+ _y_3 _returnvalue_6) _z_3) "0, 0, 0" "1,1,1") "AlwaysSpawn" 0 0)
          (Utilities|FlowControl|Sequence
            (:then_0
              (Utilities|FlowControl|Delay 2.0)
              (Actor|DestroyActor))
            (:then_1
              (Utilities|FlowControl|Sequence
                (:then_0
                  (if (not (< (Math|Random|RandomIntegerinRange 0 1) 1))
                    (Game|SpawnActorfromClass "/Game/ThirdPersonBP/Blueprints/BP_Riven.BP_Riven_C" (Math|Transform|MakeTransform (Math|Vector|MakeVector (+ _x _returnvalue_2) (+ _y _returnvalue_2) _z) "0, 0, 0" "1,1,1") "AlwaysSpawn" 0 0)))
                (:then_1
                  (if (< (Math|Random|RandomIntegerinRange 0 1) 1)
                    (Game|SpawnActorfromClass "/Game/ThirdPersonBP/Blueprints/BP_lightball.BP_lightball_C" (Math|Transform|MakeTransform (Math|Vector|MakeVector (+ _x_4 _returnvalue_8) (+ _y_4 _returnvalue_8) _z_4) "0, 0, 0" "1,1,1") "AlwaysSpawn" 0 0)
                    (if (not (< (Math|Random|RandomIntegerinRange 0 4) 4))
                      (Game|SpawnActorfromClass "/Game/ThirdPersonBP/Blueprints/BP_lightball.BP_lightball_C" (Math|Transform|MakeTransform (Math|Vector|MakeVector (+ _x_2 _returnvalue_4) (+ _y_2 _returnvalue_4) _z_2) "0, 0, 0" "1,1,1") "AlwaysSpawn" 0 0))))))))))))

(event EventTick
  (params (DeltaSeconds :type Float%20%28single-precision%29))
  ;[1 1 1] 当距离玩家范围小于155时，玩家会被攻击
  (if (not (Variables|Default|GetisDead))
    (if (< (Transformation|GetDistanceTo self (Game|Player|GetPlayerPawn 0)) 3e+02)
      (Utilities|FlowControl|DoOnce false :!label _label
        (:Completed
          (Utilities|FlowControl|Delay (Math|Random|RandomFloatinRange 1.0 3.0))
          (Collision|SetCollisionEnabled (Variables|Default|GetAttackCapsule) "QueryAndPhysics")
          (Variables|Default|SetisAttacking true)
          (Utilities|FlowControl|Delay 1.0)
          (Collision|SetCollisionEnabled (Variables|Default|GetAttackCapsule) "NoCollision")
          (Variables|Default|SetisAttacking false)
          (Utilities|FlowControl|Delay 5.0)
          (goto _label Reset)))
      (else
        (goto _label Reset)))))

(fn ConstructionScript)